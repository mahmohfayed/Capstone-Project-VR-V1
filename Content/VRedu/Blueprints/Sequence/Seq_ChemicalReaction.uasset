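; Level sequence event graph for the chemical reaction cinematic in the VR education project, apparently acetic acid with bicarbonate.
; One event plays the reaction audio cue at the world origin.
; The other events are bound to the BP_Acetic+Bicarb actor and call its custom events to change its name, restore the initial name and hide the carbo element at points in the sequence.
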(event Custom|SequenceEvent_0
  (Audio|PlaySoundatLocation "/Game/VRedu/Media/reaction_audioV3_Cue.reaction_audioV3_Cue" "0, 0, 0" "0, 0, 0" 1.0 1.0 0.0 0 0 0))

(event Custom|BP_Acetic+Bicarb_Event_3
  (params (BP_Acetic+Bicarb :type BP%20Acetic+Bicarb%20Object%20Reference))
  (Default|EventHideCarbo BP_Acetic+Bicarb))

(event Custom|BP_Acetic+Bicarb_Event_0
  (params (BP_Acetic+Bicarb :type BP%20Acetic+Bicarb%20Object%20Reference))
  (Default|EventChangeName BP_Acetic+Bicarb))

(event Custom|BP_Acetic+Bicarb_Event_1
  (params (BP_Acetic+Bicarb :type BP%20Acetic+Bicarb%20Object%20Reference))
  (Default|EventInitialName BP_Acetic+Bicarb))

(event Custom|BP_Acetic+Bicarb_Event_2
  (params (BP_Acetic+Bicarb :type BP%20Acetic+Bicarb%20Object%20Reference))
  (Default|EventInitialName BP_Acetic+Bicarb))

(event Custom|BP_Acetic+Bicarb_Event_4
  (params (BP_Acetic+Bicarb :type BP%20Acetic+Bicarb%20Object%20Reference))
  (Default|EventHideCarbo BP_Acetic+Bicarb))