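; Actor for a molecule cutscene of the acetic acid and sodium bicarbonate reaction.
; BeginPlay creates and stores a Level Sequence player, but the logic that plays it and briefly shows the plus sign is disconnected.
; Sequencer events switch the text labels from reactants to sodium acetate and water while revealing the carbon dioxide component.
; Companion events restore the reactant names and hide the carbon dioxide again.
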(event Custom|EventHideCarbo
  ;[1 1 1] Sequencer Events
  (CallFunction|EventInitialName self))

(event Custom|EventChangeName
  ;[1 1 1] Sequencer Events
  (Rendering|Components|TextRender|SetText (Variables|Default|GetAcetic) (Utilities|Text|ToText(Name) (Variables|Default|GetSodiAcet)))
  (Rendering|Components|TextRender|SetText (Variables|Default|GetSodBic) (Utilities|Text|ToText(Name) (Variables|Default|Geth20)))
  (Development|SetHiddeninGame (Variables|Default|GetCarDio) false false))

(event Custom|EventInitialName
  ;[1 1 1] Sequencer Events
  (Development|SetHiddeninGame (Variables|Default|GetCarDio) true false)
  (Rendering|Components|TextRender|SetText (Variables|Default|GetAcetic) (Utilities|Text|ToText(Name) (Variables|Default|GetAceticAcid)))
  (Rendering|Components|TextRender|SetText (Variables|Default|GetSodBic) (Utilities|Text|ToText(Name) (Variables|Default|GetSodBicar))))

(event EventBeginPlay
  ;[1 1 1] Play Sequence
  (bind _returnvalue (Sequencer|Player|CreateLevelSequencePlayer (Variables|Default|GetLevel%20Sequence)))
  (Variables|Default|SetMolecule_cutscene _returnvalue))

(fn ConstructionScript)