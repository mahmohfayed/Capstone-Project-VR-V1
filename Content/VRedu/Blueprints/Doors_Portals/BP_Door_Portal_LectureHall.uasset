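; Lecture hall portal door Blueprint with two swinging leaves that sends the player to another level.
; Each leaf has a trigger that plays a yaw timeline when a pawn enters and reverses it on exit.
; A separate trigger box saves DoorID to BP_MainGameInstance, then opens the level named by the Destination enum.
; On BeginPlay, the DestinationName text is set from DoorID.
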(event OnComponentBeginOverlap(TriggerBox)
  (params (OverlappedComponent :type Primitive%20Component%20Object%20Reference) (OtherActor :type Actor%20Object%20Reference) (OtherComp :type Primitive%20Component%20Object%20Reference) (OtherBodyIndex :type Integer) (bFromSweep :type Boolean) (SweepResult :type Hit%20Result%20Structure%20%28by%20ref%29))
  (Utilities|Casting|CastToPawn OtherActor)
  (bind _asbp_main_game_instance (Utilities|Casting|CastToBP_MainGameInstance (Game|GetGameInstance)))
  (Variables|/Game/Fundamental/Blueprints/GameInstance/BP_MainGameInstance.BP_MainGameInstance_C|SetDoor%20ID _asbp_main_game_instance (Variables|Default|GetDoorID))
  (Game|OpenLevel(byName) (Utilities|String|StringToName (Utilities|String|EnumtoString (Variables|Default|GetDestination)))))

(event OnComponentBeginOverlap(DoorLeft_Trigger)
  (params (OverlappedComponent :type Primitive%20Component%20Object%20Reference) (OtherActor :type Actor%20Object%20Reference) (OtherComp :type Primitive%20Component%20Object%20Reference) (OtherBodyIndex :type Integer) (bFromSweep :type Boolean) (SweepResult :type Hit%20Result%20Structure%20%28by%20ref%29))
  (Utilities|Casting|CastToPawn OtherActor)
  (bind _slide_open (Timeline|Rotate_Open_Left PlayFromStart)
    (:Update
      (Transformation|SetRelativeRotation (Variables|Default|GetDoorLeft) (Math|Rotator|MakeRotator 0.0 0.0 (* _slide_open (Variables|Default|GetOpen%20Left%20Amount))) false false))))

(event OnComponentEndOverlap(DoorLeft_Trigger)
  (params (OverlappedComponent :type Primitive%20Component%20Object%20Reference) (OtherActor :type Actor%20Object%20Reference) (OtherComp :type Primitive%20Component%20Object%20Reference) (OtherBodyIndex :type Integer))
  (Utilities|Casting|CastToPawn OtherActor)
  (bind _slide_open (Timeline|Rotate_Open_Left ReverseFromEnd)
    (:Update
      (Transformation|SetRelativeRotation (Variables|Default|GetDoorLeft) (Math|Rotator|MakeRotator 0.0 0.0 (* _slide_open (Variables|Default|GetOpen%20Left%20Amount))) false false))))

(event OnComponentBeginOverlap(DoorRight_Trigger)
  (params (OverlappedComponent :type Primitive%20Component%20Object%20Reference) (OtherActor :type Actor%20Object%20Reference) (OtherComp :type Primitive%20Component%20Object%20Reference) (OtherBodyIndex :type Integer) (bFromSweep :type Boolean) (SweepResult :type Hit%20Result%20Structure%20%28by%20ref%29))
  (Utilities|Casting|CastToPawn OtherActor)
  (bind _slide_open (Timeline|Rotate_Open_Right PlayFromStart)
    (:Update
      (Transformation|SetRelativeRotation (Variables|Default|GetDoorRight) (Math|Rotator|MakeRotator 0.0 0.0 (* _slide_open (Variables|Default|GetOpen%20Right%20Amount))) false false))))

(event OnComponentEndOverlap(DoorRight_Trigger)
  (params (OverlappedComponent :type Primitive%20Component%20Object%20Reference) (OtherActor :type Actor%20Object%20Reference) (OtherComp :type Primitive%20Component%20Object%20Reference) (OtherBodyIndex :type Integer))
  (Utilities|Casting|CastToPawn OtherActor)
  (bind _slide_open (Timeline|Rotate_Open_Right ReverseFromEnd)
    (:Update
      (Transformation|SetRelativeRotation (Variables|Default|GetDoorRight) (Math|Rotator|MakeRotator 0.0 0.0 (* _slide_open (Variables|Default|GetOpen%20Right%20Amount))) false false))))

(event EventBeginPlay
  (Rendering|Components|TextRender|SetText (Variables|Default|GetDestination%20Name) (CallFunction|ConvertDoorIDtoText)))

(event Collision|EventActorBeginOverlap
  (params (OtherActor :type Actor%20Object%20Reference)))

(event EventTick
  (params (DeltaSeconds :type Float%20%28single-precision%29)))

(fn ConstructionScript)

(fn ConvertDoorIDtoText
  (return (Utilities|Text|MakeLiteralText (Utilities|Text|ToText(Name) (Utilities|String|StringToName (Utilities|String|ToString(Name) (Variables|Default|GetDoorID)))))))