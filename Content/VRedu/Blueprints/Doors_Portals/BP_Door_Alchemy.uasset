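; BP_Door_Alchemy is a double door actor whose two leaves swing open when a pawn approaches and close when it leaves.
; Each leaf has its own trigger volume and timeline, so the sides operate independently.
; The timeline's SlideOpen curve, scaled by that side's open amount, sets the leaf's relative yaw.
; Begin overlap plays the timeline from the start and end overlap reverses it from the end, rather than from the current position.
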(event OnComponentBeginOverlap(DoorLeft_Trigger)
  (params (OverlappedComponent :type Primitive%20Component%20Object%20Reference) (OtherActor :type Actor%20Object%20Reference) (OtherComp :type Primitive%20Component%20Object%20Reference) (OtherBodyIndex :type Integer) (bFromSweep :type Boolean) (SweepResult :type Hit%20Result%20Structure%20%28by%20ref%29))
  (Utilities|Casting|CastToPawn OtherActor)
  (bind _slide_open (Timeline|Timeline_0 PlayFromStart)
    (:Update
      (Transformation|SetRelativeRotation (Variables|Default|GetDoorLeft) (Math|Rotator|MakeRotator 0.0 0.0 (* _slide_open (Variables|Default|GetOpenAmountLeft))) false false))))

(event OnComponentEndOverlap(DoorLeft_Trigger)
  (params (OverlappedComponent :type Primitive%20Component%20Object%20Reference) (OtherActor :type Actor%20Object%20Reference) (OtherComp :type Primitive%20Component%20Object%20Reference) (OtherBodyIndex :type Integer))
  (Utilities|Casting|CastToPawn OtherActor)
  (bind _slide_open (Timeline|Timeline_0 ReverseFromEnd)
    (:Update
      (Transformation|SetRelativeRotation (Variables|Default|GetDoorLeft) (Math|Rotator|MakeRotator 0.0 0.0 (* _slide_open (Variables|Default|GetOpenAmountLeft))) false false))))

(event OnComponentBeginOverlap(DoorRight_Trigger)
  (params (OverlappedComponent :type Primitive%20Component%20Object%20Reference) (OtherActor :type Actor%20Object%20Reference) (OtherComp :type Primitive%20Component%20Object%20Reference) (OtherBodyIndex :type Integer) (bFromSweep :type Boolean) (SweepResult :type Hit%20Result%20Structure%20%28by%20ref%29))
  (Utilities|Casting|CastToPawn OtherActor)
  (bind _slide_open (Timeline|Timeline_1 PlayFromStart)
    (:Update
      (Transformation|SetRelativeRotation (Variables|Default|GetDoorRight) (Math|Rotator|MakeRotator 0.0 0.0 (* _slide_open (Variables|Default|GetOpenAmountRight))) false false))))

(event OnComponentEndOverlap(DoorRight_Trigger)
  (params (OverlappedComponent :type Primitive%20Component%20Object%20Reference) (OtherActor :type Actor%20Object%20Reference) (OtherComp :type Primitive%20Component%20Object%20Reference) (OtherBodyIndex :type Integer))
  (Utilities|Casting|CastToPawn OtherActor)
  (bind _slide_open (Timeline|Timeline_1 ReverseFromEnd)
    (:Update
      (Transformation|SetRelativeRotation (Variables|Default|GetDoorRight) (Math|Rotator|MakeRotator 0.0 0.0 (* _slide_open (Variables|Default|GetOpenAmountRight))) false false))))

(fn ConstructionScript)