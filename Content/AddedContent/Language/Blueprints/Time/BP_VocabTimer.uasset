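; BP_VocabTimer is a minutes-and-seconds countdown actor, apparently for a vocabulary feature in the language content.
; While Enabled, Tick uses a one-second Delay as a throttle to decrement Seconds, borrowing from Minutes until both reach zero.
; BeginTimer only adds a BP_VocabTime widget to the viewport, and EndTimer clears Enabled to stop the countdown.
; Nothing in this graph sets Enabled to true or reacts when time runs out.
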(event Custom|Begin%20Timer
  (bind _returnvalue (UserInterface|CreateWidget "/Game/AddedContent/Language/Blueprints/Time/BP_VocabTime.BP_VocabTime_C"))
  (UserInterface|Viewport|AddtoViewport _returnvalue 0))

(event Custom|End%20Timer
  (Variables|Default|Setenabled false))

(event Collision|EventActorBeginOverlap
  (params (OtherActor :type Actor%20Object%20Reference)))

(event EventTick
  (params (DeltaSeconds :type Float%20%28single-precision%29))
  (if (Variables|Default|Getenabled)
    (Utilities|FlowControl|Delay 1.0)
    (if (== (Variables|Default|GetSeconds) 0)
      (if (not (== (Variables|Default|GetMinutes) 0))
        (Variables|Default|SetSeconds 59)
        (Variables|Default|SetMinutes (- (Variables|Default|GetMinutes) 1)))
      (else
        (Variables|Default|SetSeconds (- (Variables|Default|GetSeconds) 1))))))

(event EventBeginPlay)

(fn ConstructionScript)