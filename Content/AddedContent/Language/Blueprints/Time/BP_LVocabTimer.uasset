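; BP_LVocabTimer is a minutes-and-seconds countdown timer, apparently for a language vocabulary activity.
; Tick feeds a one-second Delay to decrement the time about once per second, setting TimerDone when both values reach zero.
; BeginTimer only adds the WBP_LVocabTime widget to the viewport, so the countdown runs independently of it.
; EndTimer removes all widgets without stopping the countdown.
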(event Custom|Begin%20Timer
  (bind _returnvalue (UserInterface|CreateWidget "/Game/AddedContent/Language/Blueprints/Time/WBP_LVocabTime.WBP_LVocabTime_C" 0 0))
  (UserInterface|Viewport|AddtoViewport _returnvalue 0))

(event Custom|End%20Timer
  (Viewport|RemoveAllWidgets))

(event Collision|EventActorBeginOverlap
  (params (OtherActor :type Actor%20Object%20Reference)))

(event EventTick
  (params (DeltaSeconds :type Float%20%28single-precision%29))
  (Utilities|FlowControl|Delay 1.0)
  (if (== (Variables|Default|GetSeconds) 0)
    (if (== (Variables|Default|GetMinutes) 0)
      (Variables|Default|Settimer_done true)
      (else
        (Variables|Default|SetSeconds 59)
        (Variables|Default|SetMinutes (- (Variables|Default|GetMinutes) 1))))
    (else
      (Variables|Default|SetSeconds (- (Variables|Default|GetSeconds) 1)))))

(event EventBeginPlay)

(fn ConstructionScript)