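; BP_Vocab is an actor that displays a vocabulary text in the world through five widget components, Word1 to Word5.
; On BeginPlay it creates one BP_VocabText widget from its Text variable and assigns that same instance to all five components.
; It has no other active logic, as the construction script is empty and the overlap and tick events are disabled.
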(event Collision|EventActorBeginOverlap
  (params (OtherActor :type Actor%20Object%20Reference)))

(event EventTick
  (params (DeltaSeconds :type Float%20%28single-precision%29)))

(event EventBeginPlay
  (bind _returnvalue (UserInterface|CreateWidget "/Game/AddedContent/Language/Blueprints/BP_VocabText.BP_VocabText_C" 0 (Variables|Default|GetText)))
  (UserInterface|SetWidget (Variables|Default|GetWord1) _returnvalue)
  (UserInterface|SetWidget (Variables|Default|GetWord2) _returnvalue)
  (UserInterface|SetWidget (Variables|Default|GetWord3) _returnvalue)
  (UserInterface|SetWidget (Variables|Default|GetWord4) _returnvalue)
  (UserInterface|SetWidget (Variables|Default|GetWord5) _returnvalue))

(fn ConstructionScript)