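; BP_SentenceBlockSlot is a slot in a sentence puzzle that accepts a word block and checks it against its expected word.
; When a BP_SentenceBlock overlaps the empty slot's box collision, it snaps to the box location and its text is compared to WordtoMatch.
; A match sets a correct flag and asks DisplayReference to check the answer, while a mismatch prints a debug message.
; The held block leaving clears the slot's state.
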(event OnComponentBeginOverlap(BoxCollision)
  (params (OverlappedComponent :type Primitive%20Component%20Object%20Reference) (OtherActor :type Actor%20Object%20Reference) (OtherComp :type Primitive%20Component%20Object%20Reference) (OtherBodyIndex :type Integer) (bFromSweep :type Boolean) (SweepResult :type Hit%20Result%20Structure%20%28by%20ref%29))
  ;[0.6827 0.3853 1] Center the Block
  (Utilities|IsValid (Variables|Default|GetCenteredBlock)
    (:Is%20Not%20Valid
      (bind _asbp_sentence_block (Utilities|Casting|CastToBP_SentenceBlock OtherActor))
      (Transformation|SetActorLocationAndRotation _asbp_sentence_block (.location (Transformation|GetWorldTransform (Variables|Default|GetBox%20Collision))))
      ;[0.8574 0.5546 1] Check if Block Word Matches
      (bind _output_get (Variables|Default|SetCenteredBlock _asbp_sentence_block))
      (bind _output_get_2 (Variables|Default|SetKey (Variables|/Game/AddedContent/Language/Blueprints/Vocab/BP_VocabularyBlock.BP_VocabularyBlock_C|GetBlock%20Text _output_get)))
      (if (Utilities|Enum|Equal(Enum) _output_get_2 (Variables|Default|GetWordtoMatch))
        (Variables|Default|SetCorrect_0 true)
        (Default|CheckifCorrect (Variables|Default|GetDisplayReference))
        (else
          (Development|PrintString "Not a Match" true true "(R=1.000000,G=0.000000,B=0.000000,A=1.000000)" 5.0))))))

(event OnComponentEndOverlap(BoxCollision)
  (params (OverlappedComponent :type Primitive%20Component%20Object%20Reference) (OtherActor :type Actor%20Object%20Reference) (OtherComp :type Primitive%20Component%20Object%20Reference) (OtherBodyIndex :type Integer))
  (bind _asbp_sentence_block (Utilities|Casting|CastToBP_SentenceBlock OtherActor))
  (if (== _asbp_sentence_block (Variables|Default|GetCenteredBlock))
    (Variables|Default|SetCenteredBlock 0)
    (Variables|Default|SetKey "")
    (Variables|Default|SetCorrect_0 false)))

(event Collision|EventActorBeginOverlap
  (params (OtherActor :type Actor%20Object%20Reference)))

(fn ConstructionScript
  (|CallParentFunction))