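; Translation puzzle display that shows a sentence and checks whether every word slot holds the correct block.
; On creation by a puzzle board, it sets a sentence widget and spawns a row of BP_BlockSlot actors, each given one word to match.
; When all slots are correct, it plays a coin sound and, through a resettable DoOnce, tells the board to release its pieces.
; It can also destroy its spawned slots.
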(event Custom|CheckIfCorrect
  ;[0.5086 0.7379 1] Check if All Slots Are Correct
  (bind _array_element (Utilities|Array|ForEachLoopwithBreak (Variables|Default|GetBlockSlots) :!label _label)
    (:LoopBody
      (if (Variables|/Game/AddedContent/Language/Blueprints/Puzzles/Sentences/BP_BlockSlot.BP_BlockSlot_C|GetCorrect_0 _array_element)
        (Variables|Default|SetAllCorrect true)
        (else
          (Variables|Default|SetAllCorrect false)
          (goto _label Break))))
    (:Completed
      (if (Variables|Default|GetAllCorrect)
        (Audio|PlaySound2D "/Game/AddedContent/Interface_And_Item_Sounds/WAV/Coins_15.Coins_15" 1.0 1.0 0.0 0 0)
        (Utilities|FlowControl|DoOnce false
          (:Completed
            (Default|ReleasePieces (Variables|Default|GetPuzzleBoardRef))))))))

(event Custom|CreateTranslateDisplay
  (params (Puzzle%20Board :type BP%20Puzzle%20Board%20Object%20Reference))
  (bind _blocktransform (Variables|Default|GetBlockTransform))
  (Variables|Default|SetPuzzleBoardRef Puzzle%20Board)
  (Utilities|FlowControl|Sequence
    (:then_0
      ;[1 0.8394 0.5265] Set SentenceWidget
      (bind _returnvalue (UserInterface|CreateWidget "/Game/AddedContent/Language/Blueprints/Puzzles/Sentences/WBP_Sentences.WBP_Sentences_C" 0 (Variables|Default|GetOriginalSentence)))
      (UserInterface|SetWidget (Variables|Default|GetSentenceWidget) _returnvalue))
    (:then_1
      ;[0.5521 1 1] Create Block Slots
      (for _index (range 0 (- (Utilities|Array|Length (Variables|Default|GetWordArray)) 1))
        (bind _output_get (Variables|Default|SetTranforms (Math|Transform|MakeTransform (Math|Vector|MakeVector (.x (.location _blocktransform)) (+ (.y (.location _blocktransform)) (* _index 60)) (.z (.location _blocktransform))) (.rotation _blocktransform) (.scale _blocktransform))))
        (bind _returnvalue_2 (Game|SpawnActorfromClass "/Game/AddedContent/Language/Blueprints/Puzzles/Sentences/BP_BlockSlot.BP_BlockSlot_C" _output_get "Undefined" 0 self 0 0 0))
        (Utilities|Array|Add (Variables|Default|GetBlockSlots) _returnvalue_2)
        ;[0.6461 0.7205 1] Set Word to Match
        (bind _output_get_2 (Variables|/Game/AddedContent/Language/Blueprints/Puzzles/Sentences/BP_BlockSlot.BP_BlockSlot_C|SetWordtoMatch _returnvalue_2 (Utilities|Text|ToText(String) (Utilities|Array|Get(acopy) (Variables|Default|GetWordArray) _index))))
        (Rendering|Components|TextRender|SetText (Variables|/Game/AddedContent/Language/Blueprints/Puzzles/Sentences/BP_BlockSlot.BP_BlockSlot_C|GetWordMatchText _returnvalue_2) _output_get_2) ; for editing purposes only
      ))
    (:then_2
      ;[0.5086 0.7379 1] Check if All Slots Are Correct
      (Utilities|FlowControl|DoOnce false) ; enters at Reset
    )))

(event Custom|DeleteBlockSlots
  (bind _arrayelement (Utilities|Array|ReverseforEachLoop (Variables|Default|GetBlockSlots))
    (:LoopBody
      (Actor|DestroyActor _arrayelement))))

(event EventBeginPlay)

(fn ConstructionScript)