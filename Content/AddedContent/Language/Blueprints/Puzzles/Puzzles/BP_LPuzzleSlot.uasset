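; Slot actor for a language puzzle that accepts BP_LPuzzlePiece actors and shows when the correct one is placed.
; When a piece overlaps the box collision, it is stored as the current piece and snapped to the box's location and rotation.
; If that piece's Slot value matches this slot's Piece, the cube switches to an emissive green material.
; Wrong pieces still snap, and nothing clears the state or material afterward.
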(event OnComponentBeginOverlap(BoxCollision)
  (params (OverlappedComponent :type Primitive%20Component%20Object%20Reference) (OtherActor :type Actor%20Object%20Reference) (OtherComp :type Primitive%20Component%20Object%20Reference) (OtherBodyIndex :type Integer) (bFromSweep :type Boolean) (SweepResult :type Hit%20Result%20Structure%20%28by%20ref%29))
  (bind _box_collision (Variables|Default|GetBox%20Collision))
  (bind _returnvalue (Transformation|GetWorldTransform _box_collision))
  (bind _asbp_lpuzzle_piece (Utilities|Casting|CastToBP_LPuzzlePiece OtherActor))
  (bind _output_get (Variables|Default|SetCurrentPiece _asbp_lpuzzle_piece))
  (Transformation|SetActorLocationAndRotation _asbp_lpuzzle_piece (.location _returnvalue) (.rotation _returnvalue))
  (if (== (Variables|/Game/AddedContent/Language/Blueprints/Puzzles/Puzzles/BP_LPuzzlePiece.BP_LPuzzlePiece_C|GetSlot _output_get) (Variables|Default|GetPiece))
    (Rendering|Material|SetMaterial (Variables|Default|GetCube) 0 "/Game/AddedContent/Language/Materials/M_Emissive_Green.M_Emissive_Green")))

(event EventBeginPlay)

(event Collision|EventActorBeginOverlap
  (params (OtherActor :type Actor%20Object%20Reference)))

(event EventTick
  (params (DeltaSeconds :type Float%20%28single-precision%29)))

(fn ConstructionScript)