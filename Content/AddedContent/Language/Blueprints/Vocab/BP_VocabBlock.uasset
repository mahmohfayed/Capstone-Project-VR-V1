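; Vocabulary block actor that displays a word and can be grabbed and dropped as a physics object.
; On BeginPlay it creates one BP_VocabText widget from its Text and assigns that same instance to six widget components, Word1 to Word6.
; Grab disables physics on the Cube and attaches the root to the given component, keeping world transform; Drop re-enables physics and detaches.
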(event EventBeginPlay
  (bind _returnvalue (UserInterface|CreateWidget "/Game/AddedContent/Language/Blueprints/Vocab/BP_VocabText.BP_VocabText_C" 0 (Variables|Default|GetText)))
  (UserInterface|SetWidget (Variables|Default|GetWord1) _returnvalue)
  (UserInterface|SetWidget (Variables|Default|GetWord2) _returnvalue)
  (UserInterface|SetWidget (Variables|Default|GetWord3) _returnvalue)
  (UserInterface|SetWidget (Variables|Default|GetWord4) _returnvalue)
  (UserInterface|SetWidget (Variables|Default|GetWord5) _returnvalue)
  (UserInterface|SetWidget (Variables|Default|GetWord6) _returnvalue))

(event EventGrab
  (params (AttachTo :type Scene%20Component%20Object%20Reference))
  (Physics|SetSimulatePhysics (Variables|Default|GetCube) false)
  (Transformation|AttachComponentToComponent (Variables|Transformation|GetRootComponent) AttachTo "None" "KeepWorld" "KeepWorld" "KeepWorld" false))

(event EventDrop
  (Physics|SetSimulatePhysics (Variables|Default|GetCube) true)
  (Transformation|DetachFromActor "KeepWorld" "KeepWorld" "KeepWorld"))

(fn ConstructionScript)