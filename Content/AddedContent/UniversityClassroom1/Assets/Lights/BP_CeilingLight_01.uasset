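; BP_CeilingLight_01 is a configurable ceiling light fixture for the university classroom environment, pairing a mesh with a spotlight.
; The construction script checks the Lit flag; when on, it applies the exposed intensity, indirect intensity, cone angle, radius and temperature settings to the spotlight.
; When off, it zeroes the attenuation radius instead, and both branches set the mesh's first material slot.
; It has no active runtime logic.
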(event EventBeginPlay)

(event Collision|EventActorBeginOverlap
  (params (OtherActor :type Actor%20Object%20Reference)))

(event EventTick
  (params (DeltaSeconds :type Float%20%28single-precision%29)))

(fn ConstructionScript
  (bind _ceilinglightsunk_01 (Variables|Default|GetCeilingLightSunk_01))
  (bind _spotlight1 (Variables|Default|GetSpotLight1))
  (if (Variables|Default|GetLit)
    (Class|LightComponent|SetIndirectLightingIntensity _spotlight1 (Variables|Default|GetIndirect%20Intensity))
    (Rendering|Lighting|SetInnerConeAngle _spotlight1 (Variables|Range|GetInner%20Cone%20Range))
    (Rendering|Lighting|SetOuterConeAngle _spotlight1 (Variables|Range|GetOuter%20Cone%20Range))
    (Rendering|Lighting|SetAttenuationRadius _spotlight1 (Variables|Range|GetRadius))
    (Rendering|Components|Light|SetIntensity _spotlight1 (Variables|Default|GetIntensity))
    (Class|LightComponent|SetTemperature _spotlight1 (Variables|Default|GetTemperature))
    (Rendering|Material|SetMaterial _ceilinglightsunk_01 0 0)
    (else
      (Rendering|Lighting|SetAttenuationRadius _spotlight1 0.0)
      (Rendering|Lighting|SetAttenuationRadius _spotlight1 0.0)
      (Rendering|Material|SetMaterial _ceilinglightsunk_01 0 0))))